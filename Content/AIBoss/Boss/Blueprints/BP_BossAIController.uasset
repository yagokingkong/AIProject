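; AI controller for the boss that starts its behavior tree on BeginPlay and tracks the player through AI perception.
; Perception updates go to HandleSightSense, which reacts only to sight stimuli from the player character.
; It sets TargetActor and CanSeePlayer on the blackboard while the player is seen.
; On losing sight it clears both and stores the stimulus position as LastKnownLocation.
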(event `self.ReceiveBeginPlay`
  (`self.RunBehaviorTree` "/Game/AIBoss/Boss/Tasks/BT_Boss.BT_Boss"))

(event `self.AIPerception.OnTargetPerceptionUpdated`
  (params (Actor :type "Actor Object Reference") (Stimulus :type "AIStimulus Structure"))
  (`self.HandleSightSense` Actor Stimulus))

(fn `HandleSightSense`
  (params (Actor :type "Actor Object Reference") (Stimulus :type "AIStimulus Structure"))
  (bind (_stimulus_age _stimulus_expirationage _stimulus_strength _stimulus_stimuluslocation _stimulus_receiverlocation _stimulus_tag _stimulus_bsuccessfullysensed) (break `AIStimulus` (`local.Stimulus`)))
  ;[0 0 0] Setting The blackboard values for the AI's behavior tree.
  (bind _returnvalue (`AIPerceptionSystem.GetSenseClassForStimulus` Stimulus))
  (if (== _returnvalue "/Script/AIModule.AISense_Sight")
    (if (== (`local.Actor`) (`GameplayStatics.GetPlayerCharacter` 0))
      (`BlackboardComponent.SetValueAsObject` (`self.Blackboard`) "TargetActor" (`KismetMathLibrary.SelectObject` (`GameplayStatics.GetPlayerCharacter` 0) null _stimulus_bsuccessfullysensed))
      (if _stimulus_bsuccessfullysensed
        (`BlackboardComponent.SetValueAsBool` (`self.Blackboard`) "CanSeePlayer" true)
        (else
          (`BlackboardComponent.SetValueAsVector` (`self.Blackboard`) "LastKnownLocation" _stimulus_stimuluslocation)
          (`BlackboardComponent.SetValueAsBool` (`self.Blackboard`) "CanSeePlayer" false)))
      (else
        (return)))
    (else
      (return))))

(fn `UserConstructionScript`)