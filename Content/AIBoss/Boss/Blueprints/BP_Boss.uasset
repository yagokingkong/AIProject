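; Boss character that attacks the player with random melee montages, thrown rocks and fireballs.
; Montage notifies trigger melee camera shake and launch socket-spawned projectiles along SuggestProjectileVelocity arcs aimed at the player.
; During throws it disables movement and Tick turns it toward the player, until the notify restores walking.
; SphereCheck overlaps set CharacterIsInThrowRange, which is true once the player leaves the sphere.
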(event `/Game/AIBoss/Boss/Blueprints/BPI_Combat.MeleeAttack`
  (params (Target :type "Actor Object Reference"))
  ;[0 0 0] PrimaryAttack
  (`|ExecutionSequence`
    (:`then_0`
      (`|PlayMontage` (`self.Mesh`) (`|GetArrayItem` (`self.ArrayOfMontages`) (`KismetMathLibrary.RandomIntegerInRange` 0 6))
        (:`then`
          (`KismetSystemLibrary.PrintString` "MeleeAttack"))
        (:`OnNotifyBegin`
          (`GameplayStatics.PlayWorldCameraShake` "/Game/AIBoss/Boss/Blueprints/BP_CameraShake.BP_CameraShake_C" (`self.K2_GetActorLocation` (`GameplayStatics.GetPlayerCharacter` 0)) 1000.0 1000.0))))))

(event `self.ReceiveTick`
  (params (DeltaSeconds :type "Float (single-precision)"))
  ;[0 0 0] Throw Attack condition check
  (if (or (`self.bThrowRockAttack`) (`self.ThrowFireBallAttack`))
    (`self.K2_SetActorRotation` (`KismetMathLibrary.FindLookAtRotation` (`self.K2_GetActorLocation` self) (`self.K2_GetActorLocation` (`GameplayStatics.GetPlayerCharacter` 0))))))

(event `self.SphereCheck.OnComponentBeginOverlap`
  (params (OverlappedComponent :type "PrimitiveComponent Object Reference") (OtherActor :type "Actor Object Reference") (OtherComp :type "PrimitiveComponent Object Reference") (OtherBodyIndex :type Integer) (bFromSweep :type Boolean) (SweepResult :type "HitResult Structure (by ref)"))
  ;[0 0 0] RockAttack Depends on this code
  (bind _asbp_third_person_character (cast `/Game/ThirdPerson/Blueprints/BP_ThirdPersonCharacter` OtherActor))
  (set `self.ThirdPersonCharRef` _asbp_third_person_character)
  (set `self.bCharacterIsInThrowRange` false))

(event `self.SphereCheck.OnComponentEndOverlap`
  (params (OverlappedComponent :type "PrimitiveComponent Object Reference") (OtherActor :type "Actor Object Reference") (OtherComp :type "PrimitiveComponent Object Reference") (OtherBodyIndex :type Integer))
  ;[0 0 0] RockAttack Depends on this code
  (cast `/Game/ThirdPerson/Blueprints/BP_ThirdPersonCharacter` OtherActor)
  (set `self.bCharacterIsInThrowRange` true))

(event `/Game/AIBoss/Boss/Blueprints/BPI_Combat.ThrowRockAttack`
  (params (Target :type "Actor Object Reference"))
  (bind _spawnedrockref (`self.SpawnedRockRef`))
  (bind _charactermovement (`self.CharacterMovement`))
  (bind (_returnvalue_x _returnvalue_y _returnvalue_z) (`KismetMathLibrary.BreakVector` (`self.K2_GetActorLocation` (`GameplayStatics.GetPlayerCharacter` 0))))
  (bind _projectilemovement (`/Game/AIBoss/Boss/Blueprints/BP_Rock.ProjectileMovement` _spawnedrockref))
  ;[0 0 0] ThrowAttack
  (bind _asbp_boss (cast `/Game/AIBoss/Boss/Blueprints/BP_Boss` Target))
  (set `self.bThrowRockAttack` true)
  (`CharacterMovementComponent.DisableMovement` _charactermovement)
  (`MovementComponent.StopMovementImmediately` _charactermovement)
  (`|PlayMontage` (`self.Mesh`) "/Game/AIBoss/Boss/Animations/Boss_Throw_Montage.Boss_Throw_Montage" 1.0 0.0 "None"
    (:`then`
      (`KismetSystemLibrary.Delay` 0.3)
      (bind (_returnvalue_x_2 _returnvalue_y_2 _returnvalue_z_2) (`KismetMathLibrary.BreakVector` (`self.K2_GetActorLocation` _asbp_boss)))
      (bind _returnvalue (`|SpawnActorFromClass` "/Game/AIBoss/Boss/Blueprints/BP_Rock.BP_Rock_C" (`KismetMathLibrary.MakeTransform` (`KismetMathLibrary.MakeVector` _returnvalue_x_2 _returnvalue_y_2 (- _returnvalue_z_2 (`CapsuleComponent.GetScaledCapsuleHalfHeight` (`Character.CapsuleComponent` _asbp_boss)))) (`self.K2_GetActorRotation` _asbp_boss)) "AdjustIfPossibleButAlwaysSpawn" "OverrideRootScale" null _asbp_boss))
      (bind _output_get (set `self.SpawnedRockRef` _returnvalue))
      (`self.K2_AttachToComponent` _output_get (`Character.Mesh` _asbp_boss) "Emote_Skull" "SnapToTarget" "KeepRelative" "KeepRelative" true))
    (:`OnNotifyBegin`
      (bind _output_get_2 (set `self.TargetLoc` (`KismetMathLibrary.MakeVector` _returnvalue_x _returnvalue_y (- _returnvalue_z -60.0))))
      (bind _tossvelocity (`GameplayStatics.BlueprintSuggestProjectileVelocity` (`self.K2_GetActorLocation` _spawnedrockref) _output_get_2 6000.0 0.0 "DoNotTrace" 100.0))
      (`self.K2_SetActorRotation` (`KismetMathLibrary.FindLookAtRotation` (`self.K2_GetActorLocation` self) _output_get_2))
      (`self.K2_SetActorRotation` _spawnedrockref (`KismetMathLibrary.Conv_VectorToRotator` _output_get_2) false)
      (`self.K2_DetachFromActor` _spawnedrockref "KeepWorld" "KeepWorld" "KeepWorld")
      (set `MovementComponent.Velocity` _tossvelocity _projectilemovement)
      (`ActorComponent.Activate` _projectilemovement false)
      (set `self.bThrowRockAttack` false)
      (`CharacterMovementComponent.SetMovementMode` (`self.CharacterMovement`) "MOVE_Walking" 0))))

(event `/Game/AIBoss/Boss/Blueprints/BPI_Combat.FireBallAttack`
  (params (Target :type "Actor Object Reference"))
  (bind _spawnedfireballref (`self.SpawnedFireBallRef`))
  (bind (_returnvalue_x _returnvalue_y _returnvalue_z) (`KismetMathLibrary.BreakVector` (`self.K2_GetActorLocation` (`GameplayStatics.GetPlayerCharacter` 0))))
  (bind _projectilemovement (`/Game/AIBoss/Boss/Blueprints/BP_FireBall.ProjectileMovement` _spawnedfireballref))
  ;[0 0 0] FireBallAttack
  (bind _asbp_boss (cast `/Game/AIBoss/Boss/Blueprints/BP_Boss` Target))
  (set `self.ThrowFireBallAttack` true)
  (bind _charactermovement (`Character.CharacterMovement` _asbp_boss))
  (`CharacterMovementComponent.DisableMovement` _charactermovement)
  (`MovementComponent.StopMovementImmediately` _charactermovement)
  (`|PlayMontage` (`self.Mesh`) "/Game/AIBoss/Boss/Animations/FireBall_Montage.FireBall_Montage"
    (:`OnNotifyBegin`
      (bind _returnvalue (`|SpawnActorFromClass` "/Game/AIBoss/Boss/Blueprints/BP_FireBall.BP_FireBall_C" (`SceneComponent.GetSocketTransform` (`self.Mesh`) "FireBallSocket" "RTS_World") "Undefined" "OverrideRootScale" null null))
      (set `self.SpawnedFireBallRef` _returnvalue)
      (bind _output_get (set `self.TargetLoc` (`KismetMathLibrary.MakeVector` _returnvalue_x _returnvalue_y (- _returnvalue_z -75.0))))
      (bind _tossvelocity (`GameplayStatics.BlueprintSuggestProjectileVelocity` (`self.K2_GetActorLocation` _spawnedfireballref) _output_get 3000.0 0.0 "DoNotTrace" 100.0))
      (`self.K2_SetActorRotation` (`KismetMathLibrary.FindLookAtRotation` (`self.K2_GetActorLocation` self) _output_get))
      (`self.K2_SetActorRotation` _spawnedfireballref (`KismetMathLibrary.Conv_VectorToRotator` _output_get) false)
      (set `MovementComponent.Velocity` _tossvelocity _projectilemovement)
      (`ActorComponent.Activate` _projectilemovement false)
      (set `self.ThrowFireBallAttack` false)
      (`CharacterMovementComponent.SetMovementMode` (`self.CharacterMovement`) "MOVE_Walking" 0)
      (`PrimitiveComponent.SetCollisionResponseToAllChannels` (`/Game/AIBoss/Boss/Blueprints/BP_FireBall.Sphere` (`self.SpawnedFireBallRef`)) "ECR_Block"))))

(fn `CalculateProjectilePoint`
  (params (ProjectileMovementRef :type "ProjectileMovementComponent Object Reference"))
  (returns (CalculatedVelocity :type "Vector Structure"))
  (bind _tossvelocity (`GameplayStatics.BlueprintSuggestProjectileVelocity` (`self.K2_GetActorLocation` (`ActorComponent.GetOwner` ProjectileMovementRef)) (`self.K2_GetActorLocation` (`GameplayStatics.GetPlayerCharacter` 0)) 2000.0 0.0 "DoNotTrace"))
  (return _tossvelocity))

(fn `UserConstructionScript`)